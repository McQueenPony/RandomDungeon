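; BP_Challenge_2 is a challenge room for the program-generated dungeon, stocked with arrow and lurker traps.
; Its construction script fills the Traps map, pairing BP_Arrow and BP_Luker each with a MakeTrapMap-built list of entries.
; The LighttheRoad event reveals StaticMesh5, and BeginPlay, overlap and Tick are left empty.
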(event EventBeginPlay)

(event Collision|EventActorBeginOverlap
  (params (OtherActor :type Actor%20Object%20Reference)))

(event EventTick
  (params (DeltaSeconds :type Float%20%28single-precision%29)))

(event EventLighttheRoad
  (Rendering|SetVisibility (Variables|Default|GetStaticMesh5) true false))

(fn ConstructionScript
  (Utilities|Map|Add (Variables|Default|GetTraps) "/Game/ProgramGeneratedDungeon/Fillings/BP_Arrow.BP_Arrow_C" (Utilities|Struct|MakeTrapMap (Utilities|Array|MakeArray 0 0 0 0 0 0 0)))
  (Utilities|Map|Add (Variables|Default|GetTraps) "/Game/ProgramGeneratedDungeon/Fillings/BP_Luker.BP_Luker_C" (Utilities|Struct|MakeTrapMap (Utilities|Array|MakeArray 0 0 0))))