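; BP_Challenge_1 is a challenge room for the program-generated dungeon, defining its trap layout and a road-lighting event.
; MakeTrapMap fills the Traps map, keying the arrow and Luker trap classes to their own groups of scene components placed in the room.
; LighttheRoad reveals a single static mesh.
; The room only supplies this data and visual hook, with no spawning logic, active Tick or construction logic of its own.
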(event EventBeginPlay)

(event Collision|EventActorBeginOverlap
  (params (OtherActor :type Actor%20Object%20Reference)))

(event EventTick
  (params (DeltaSeconds :type Float%20%28single-precision%29)))

(event EventLighttheRoad
  (Rendering|SetVisibility (Variables|Default|GetStaticMesh1) true false))

(event EventMakeTrapMap
  (Utilities|Map|Add (Variables|Default|GetTraps) "/Game/ProgramGeneratedDungeon/Fillings/BP_Arrow.BP_Arrow_C" (Utilities|Struct|MakeTrapMap (Utilities|Array|MakeArray (Variables|Default|GetScene1) (Variables|Default|GetScene2) (Variables|Default|GetScene4) (Variables|Default|GetScene3) (Variables|Default|GetScene5) (Variables|Default|GetScene6) (Variables|Default|GetScene))))
  (Utilities|Map|Add (Variables|Default|GetTraps) "/Game/ProgramGeneratedDungeon/Fillings/BP_Luker.BP_Luker_C" (Utilities|Struct|MakeTrapMap (Utilities|Array|MakeArray (Variables|Default|GetScene8) (Variables|Default|GetScene9) (Variables|Default|GetScene7)))))

(fn ConstructionScript)